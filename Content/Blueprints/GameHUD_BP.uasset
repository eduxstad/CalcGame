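; GameHUD_BP is a HUD Blueprint that draws a custom mouse cursor using the Cursor_brown texture.
; Its DrawHUD event reads the mouse position from player controller 0 and draws the texture as a small fixed-size square centered on that point.
; The position is shifted by the difference between the HUD draw size and the controller's viewport size.
; All other events and the construction script are empty.
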(event `self.ReceiveDrawHUD`
  (params (SizeX :type Integer) (SizeY :type Integer))
  (bind _returnvalue (`GameplayStatics.GetPlayerController` 0))
  (bind _returnvalue_2 (/ 30.0 2.0))
  (bind (_sizex _sizey) (`PlayerController.GetViewportSize` _returnvalue))
  (bind (_locationx _locationy) (`PlayerController.GetMousePosition` _returnvalue))
  (`self.DrawTexture` "/Game/Textures/ui/cursor_brown.cursor_brown" (- (+ _locationx (`KismetMathLibrary.Conv_IntToDouble` (- SizeX _sizex))) _returnvalue_2) (- (+ (`KismetMathLibrary.Conv_IntToDouble` (- SizeY _sizey)) _locationy) _returnvalue_2) 30.0 30.0))

(fn `UserConstructionScript`)
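; Clickable door Blueprint that lets the player move to the next room once the current room's problem is solved.
; On click it checks SolvedRoomProblem on the cached Hero_BP; if unsolved, it replaces any prior MessageUI2 widget with a hint.
; If solved, the first click swaps sprites to show the door open.
; A later click teleports the player to Destination, resets the solved flag, and optionally sets the End flag.
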(event `self.ReceiveBeginPlay`
  (bind _ashero_bp (cast `/Game/Characters/Hero_BP` (`GameplayStatics.GetPlayerCharacter` 0)))
  (set `self.PlayerCharacter` _ashero_bp))

(event `self.ReceiveActorOnClicked`
  (params (ButtonPressed :type "Key Structure" :default "AnyKey"))
  (if (`/Game/Characters/Hero_BP.SolvedRoomProblem` (`self.PlayerCharacter`))
    (if (`self.Unlocked`)
      ;[1 1 1] Move to Next Room
      (`self.K2_SetActorLocation` (`GameplayStatics.GetPlayerCharacter` 0) (`KismetMathLibrary.MakeVector` (.x (`self.K2_GetActorLocation` (`self.Destination`))) 20.0 (.z (`self.K2_GetActorLocation` (`self.Destination`)))) false true)
      (set `/Game/Characters/Hero_BP.SolvedRoomProblem` false (`self.PlayerCharacter`))
      (if (`self.TriggerEnd`)
        (set `/Game/Characters/Hero_BP.End` true (`self.PlayerCharacter`)))
      (else
        ;[1 1 1] Open Door
        (`SceneComponent.SetVisibility` (`self.roguelikeSheet_transparent__32`) false false)
        (`SceneComponent.SetVisibility` (`self.PaperSprite`) true false)
        (set `self.Unlocked` true)))
    (else
      (bind _returnvalue (`|CreateWidget` "/Game/UI/MessageUI2.MessageUI2_C" null "You need to find and solve the problem first!"))
      (`Widget.RemoveFromParent` (`self.UInstance`))
      (bind _output_get (set `self.UInstance` _returnvalue))
      (`UserWidget.AddToViewport` _output_get 0))))

(fn `UserConstructionScript`)